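; Player-controlled marine pawn for a top-down-style alien shooter, with movement, aiming, shooting, health, a kill counter and a HUD widget.
; Tick turns the control rotation toward smoothed mouse velocity or thumbstick direction, switching on the last key's device and ignoring deadzone input.
; Firing loops a timed hitscan trace from the muzzle socket, applying damage and impact effects.
; Wheel, keys and D-pad zoom the spring arm; health reaching exactly zero triggers death.
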(event EventBeginPlay
  ;[1 1 1] HUD
  (CallFunction|HUDSetup))

(event Collision|EventActorBeginOverlap
  (params (OtherActor :type Actor%20Object%20Reference)))

(event EventTick
  (params (DeltaSeconds :type Float%20%28single-precision%29))
  ;[1 1 1] Rotation/GamepadCheck
  (Marine|RotatePlayer))

(event Game|Damage|EventAnyDamage
  (params (Damage :type Float%20%28single-precision%29) (DamageType :type Damage%20Type%20Object%20Reference) (InstigatedBy :type Controller%20Object%20Reference) (DamageCauser :type Actor%20Object%20Reference))
  ;[1 1 1] Damage/Death
  (bind _outcome (Marine|DecreaseHealth Damage))
  (Marine|PlayerDeath _outcome))

(event Input|ActionEvents|InputActionFireWeapon
  (params (Key :type Key%20Structure :default "None"))
  ;[1 1 1] FireWeapon
  (:Pressed
    (Weapon|StartFiringWeapon))
  (:Released
    (Weapon|StopFiringWeapon)))

(event Input|AxisEvents|InputAxisForward/Backward
  (params (AxisValue :type Float%20%28single-precision%29))
  ;[1 1 1] PlayerMovement
  (if (Marine|IsAlive)
    (Pawn|Input|AddMovementInput "1.000000, 0, 0" AxisValue false)))

(event Input|AxisEvents|InputAxisLeft/Right
  (params (AxisValue :type Float%20%28single-precision%29))
  ;[1 1 1] PlayerMovement
  (if (Marine|IsAlive)
    (Pawn|Input|AddMovementInput "1.000000,1.000000, 0" AxisValue false)))

(event Input|KeyboardEvents|AnyKey
  (params (Key :type Key%20Structure :default "None"))
  ;[1 1 1] Rotation/GamepadCheck
  (:Pressed
    (Variables|Default|SetGamepadActive (Class|KismetInputLibrary|KeyIsGamepadKey Key))))

(event Input|KeyboardEvents|Add
  (params (Key :type Key%20Structure :default "None"))
  ;[1 1 1] CameraZoom
  (:Pressed
    (ArmLength|IncreaseArmLengthDistance)))

(event Input|KeyboardEvents|Subtract
  (params (Key :type Key%20Structure :default "None"))
  ;[1 1 1] CameraZoom
  (:Pressed
    (ArmLength|DecreaseArmLengthDistance)))

(event Input|MouseEvents|MouseWheelUp
  (params (Key :type Key%20Structure :default "None"))
  ;[1 1 1] CameraZoom
  (:Pressed
    (if (Variables|ArmLength|GetArmLengthInvert)
      (ArmLength|IncreaseArmLengthDistance)
      (else
        (ArmLength|DecreaseArmLengthDistance)))))

(event Input|MouseEvents|MouseWheelDown
  (params (Key :type Key%20Structure :default "None"))
  ;[1 1 1] CameraZoom
  (:Pressed
    (if (Variables|ArmLength|GetArmLengthInvert)
      (ArmLength|DecreaseArmLengthDistance)
      (else
        (ArmLength|IncreaseArmLengthDistance)))))

(event Input|GamepadEvents|GamepadDPadUp
  (params (Key :type Key%20Structure :default "None"))
  ;[1 1 1] CameraZoom
  (:Pressed
    (if (Variables|ArmLength|GetArmLengthInvert)
      (ArmLength|IncreaseArmLengthDistance)
      (else
        (ArmLength|DecreaseArmLengthDistance)))))

(event Input|GamepadEvents|GamepadDPadDown
  (params (Key :type Key%20Structure :default "None"))
  ;[1 1 1] CameraZoom
  (:Pressed
    (if (Variables|ArmLength|GetArmLengthInvert)
      (ArmLength|DecreaseArmLengthDistance)
      (else
        (ArmLength|IncreaseArmLengthDistance)))))

(fn ConstructionScript)

(fn RotatePlayer
  (if (Marine|IsAlive)
    (if (Variables|Default|GetGamepadActive)
      (ThumbstickInput|UpdateThumbstickAim)
      (else
        (MouseInput|UpdateMouseAim)))))

(fn DeadzoneCheck
  (return (> (Math|Vector2D|Vector2DLength (Math|Vector2D|MakeVector2D (Input|AxisValues|GetPlayerControllerUp) (Input|AxisValues|GetPlayerControllerRight))) (Variables|ThumbstickInput|GetThumbstickDeadzone))))

(fn GetMouseVelocity
  (bind _returnvalue (Game|GetPlayerController 0))
  (bind (_deltax _deltay) (Class|PlayerController|GetInputMouseDelta _returnvalue))
  (return (/ (Math|Vector2D|MakeVector2D _deltax _deltay) (Utilities|Time|GetWorldDeltaSeconds))))

(fn MouseDeadzoneCheck
  (return (> (Math|Vector2D|Vector2DLength (MouseInput|GetMouseVelocity)) (Variables|MouseInput|GetMouseDeadzone))))

(fn UpdateMouseAim
  (if (MouseInput|MouseDeadzoneCheck)
    (Pawn|SetControlRotation (Game|GetPlayerController 0) (MouseInput|GetMouseAimDirection))))

(fn UpdateThumbstickAim
  (if (ThumbstickInput|DeadzoneCheck)
    (Pawn|SetControlRotation (Game|GetPlayerController 0) (ThumbstickInput|GetThumbstickAimDirection))))

(fn GetMouseAimDirection
  (bind _returnvalue (MouseInput|GetMouseVelocity))
  (return (Math|Interpolation|RInterpTo (Pawn|GetControlRotation (Game|GetPlayerController 0) :!class /Script/Engine.Controller) (Math|Rotator|MakeRotator 0.0 0.0 (Class|KismetMathLibrary|DegAtan2 (.x _returnvalue) (.y _returnvalue))) (Utilities|Time|GetWorldDeltaSeconds) (Variables|MouseInput|GetMouseSmoothing))))

(fn GetThumbstickAimDirection
  (return (Math|Rotator|MakeRotator 0.0 0.0 (Class|KismetMathLibrary|DegAtan2 (Input|AxisValues|GetPlayerControllerRight) (Input|AxisValues|GetPlayerControllerUp)))))

(fn StartFiringWeapon
  (if (Marine|IsAlive)
    (Components|Activation|Activate (Variables|Default|GetP_AssaultRifle_MF) false)
    (bind _returnvalue (Audio|SpawnSoundatLocation "/Game/Sounds/Weapon_AssaultRifle/Stereo/RifleFire_Cue.RifleFire_Cue" (Transformation|GetActorLocation) "0, 0, 0" 1.0 1.0 0.0 0 0))
    (Variables|Default|SetRifleShot _returnvalue)
    (WeaponTracing|WeaponTrace)
    (Utilities|Time|SetTimerbyFunctionName 0 (Variables|Default|GetWeaponTraceVar) (Variables|Default|GetWeaponFiringRate) true)))

(fn StopFiringWeapon
  (if (Utilities|IsValid (Variables|Default|GetRifleShot))
    (Components|Activation|Deactivate (Variables|Default|GetP_AssaultRifle_MF))
    (Audio|Components|Audio|Stop (Variables|Default|GetRifleShot))
    (Utilities|Time|ClearTimerbyFunctionName 0 (Variables|Default|GetWeaponTraceVar))
    (if (Marine|IsAlive)
      (Audio|SpawnSoundatLocation "/Game/Sounds/Weapon_AssaultRifle/Stereo/RifleFireEnd_Cue.RifleFireEnd_Cue" (Transformation|GetActorLocation) "0, 0, 0" 1.0 1.0 0.0 0 0))))

(fn IncreaseArmLengthDistance
  (bind _springarm (Variables|Default|GetSpringArm))
  (Variables|/Script/Engine.SpringArmComponent|SetTargetArmLength _springarm (+ (Variables|/Script/Engine.SpringArmComponent|GetTargetArmLength _springarm) (Variables|ArmLength|GetTargetArmLengthZoom))))

(fn DecreaseArmLengthDistance
  (bind _springarm (Variables|Default|GetSpringArm))
  (Variables|/Script/Engine.SpringArmComponent|SetTargetArmLength _springarm (- (Variables|/Script/Engine.SpringArmComponent|GetTargetArmLength _springarm) (Variables|ArmLength|GetTargetArmLengthZoom))))

(fn IsAlive
  (return (not (Variables|PlayerStats|GetDead))))

(fn DecreaseHealth
  (params (Health :type Float%20%28single-precision%29))
  (bind _output_get (Variables|PlayerStats|SetMarineHealth (- (Variables|PlayerStats|GetMarineHealth) Health)))
  (return _output_get))

(fn AliveDebug
  (if (Marine|IsAlive)
    (Development|PrintString "Player is alive.")
    (else
      (Development|PrintString "Player is not alive."))))

(fn PlayerDeath
  (params (PlayerHealth :type Float%20%28single-precision%29))
  (if (== PlayerHealth 0.0)
    (Variables|PlayerStats|SetDead true)
    (Weapon|StopFiringWeapon)
    (Components|Animation|PlayAnimation (Variables|Character|GetMesh) "/Game/Characters/Marine/Animations/Death.Death" false)))

(fn WeaponTrace
  (bind _outhit (Collision|LineTraceByChannel (WeaponTracing|GetLineTraceStartLocation) (WeaponTracing|GetLineTraceEndLocation) "TraceTypeQuery1" false 0 "None"))
  (if (.bBlockingHit (Collision|BreakHitResult _outhit))
    (CallFunction|ImpactParticles (.Location (Collision|BreakHitResult _outhit)))
    (CallFunction|DamageAlien (.HitActor (Collision|BreakHitResult _outhit)))))

(fn GetLineTraceStartLocation
  (return (Transformation|GetSocketLocation (Variables|Default|GetWeapon) "MuzzleFlashSocket")))

(fn GetLineTraceEndLocation
  (return (+ (WeaponTracing|GetLineTraceStartLocation) (* (Math|Vector|GetForwardVector (Pawn|GetControlRotation :!class /Script/Engine.Pawn)) (Variables|LineTrace|GetLineTraceRange)))))

(fn IncreaseSpiderKill
  (Variables|PlayerStats|SetMarineKills (+ (Variables|PlayerStats|GetMarineKills) 1)))

(fn HUDSetup
  (bind _returnvalue (UserInterface|CreateWidget "/Game/UI/Widgets/HUD_Widget.HUD_Widget_C" 0 self))
  (UserInterface|Viewport|AddtoViewport _returnvalue 0))

(fn DamageAlien
  (params (Alien :type Actor%20Object%20Reference))
  (Game|Damage|ApplyDamage Alien (Variables|Default|GetAlienDam) 0 0))

(fn ImpactParticles
  (params (Location :type Vector))
  (Effects|SpawnEmitteratLocation "/Game/Effects/Weapons/Impacts/P_AssaultRifle_IH.P_AssaultRifle_IH" Location))