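; Game mode that runs escalating waves of spider aliens, starting shortly after play begins in windowed mode.
; Each wave scales the spawn count by a multiplier, and a looping timer spawns BP_Spider actors at random TargetPoints until none remain.
; RegisterAlienDeath removes spiders from the tracked array, and after a short delay the next wave starts once all have spawned and died.
; Tick prints the remaining spawn count on screen.
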(event Custom|Spawn%20Wave
  (CallFunction|SpawnAliens))

(event Custom|End%20Wave
  (Utilities|FlowControl|Delay 5.0)
  (CallFunction|IncreaseWave))

(event EventBeginPlay
  (CallFunction|Fullscreen)
  (Utilities|FlowControl|Delay 5.0)
  (CallFunction|IncreaseWave))

(event EventTick
  (params (DeltaSeconds :type Float%20%28single-precision%29))
  (Development|PrintString (Utilities|String|ToString(Integer) (Variables|Default|GetAlienSpawnRemaining))))

(fn ConstructionScript)

(fn IncreaseWave
  (Math|Integer|IncrementInt (Variables|Default|GetCurrentWave)
    (:%20%20
      (CallFunction|IncrementDifficulty)
      (Utilities|Time|SetTimerbyFunctionName 0 "Spawn Wave" 0.5 true))))

(fn SpawnAliens
  (bind _randompoint (CallFunction|GetRandomPoint))
  (Utilities|IsValid _randompoint
    (:Is%20Valid
      (bind _returnvalue (Game|SpawnActorfromClass "/Game/Blueprints/AI/BP_Spider.BP_Spider_C" (Transformation|GetActorTransform _randompoint) "Undefined" 0 0))
      (Utilities|IsValid _returnvalue
        (:Is%20Valid
          (Utilities|Array|Add (Variables|Default|GetAliens) _returnvalue)
          (bind _result (Math|Integer|DecrementInt (Variables|Default|GetAlienSpawnRemaining))
            (:%20%20
              (if (== _result 0)
                (Utilities|Time|ClearTimerbyFunctionName 0 "Spawn Wave")))))))
    (:Is%20Not%20Valid
      (Development|PrintString ":("))))

(fn GetRandomPoint
  (bind _outactors (Actor|GetAllActorsOfClass "/Script/Engine.TargetPoint"))
  (return (Utilities|Array|Get(acopy) _outactors (Math|Random|RandomIntegerinRange 0 (Utilities|Array|LastIndex _outactors)))))

(fn RegisterAlienDeath
  (params (Alien :type BP%20Spider%20Object%20Reference%20%28by%20ref%29))
  (Utilities|Array|RemoveItem (Variables|Default|GetAliens) Alien)
  (if (CallFunction|CurrentWaveCompleted)
    (CallFunction|EndWave)))

(fn CurrentWaveCompleted
  (return (and (== (Utilities|Array|Length (Variables|Default|GetAliens)) 0) (== (Variables|Default|GetAlienSpawnRemaining) 0))))

(fn IncrementDifficulty
  (bind _output_get (Variables|Default|SetDifficultyAmount (Math|Float|Round (* (Variables|Default|GetDifficultyAmount) (Variables|Default|GetDifficultyMultiplier)))))
  (Variables|Default|SetAlienSpawnRemaining _output_get))

(fn Fullscreen
  (bind _returnvalue (Settings|GetGameUserSettings))
  (Class|GameUserSettings|SetFullscreenMode _returnvalue "Windowed"))