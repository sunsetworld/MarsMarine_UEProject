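; BP_Spider is an enemy AI character that chases the player, attacks at close range and can be killed.
; A repeating AI Move To targets the player controller, while Tick checks range to pause movement and play an attack montage.
; AttackPlayer applies damage but is not called within this Blueprint.
; Incoming damage reduces health until death disables movement and collision, then after a delay credits the marine's spider kill count and destroys the actor.
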(event EventBeginPlay
  (bind _asbp_marine (Utilities|Casting|CastToBP_Marine (Game|GetPlayerCharacter 0)))
  (Variables|Default|SetBP%20Marine _asbp_marine)
  (Utilities|MovetoPlayer))

(event Collision|EventActorBeginOverlap
  (params (OtherActor :type Actor%20Object%20Reference)))

(event EventTick
  (params (DeltaSeconds :type Float%20%28single-precision%29))
  (Utilities|AttackMontage))

(event Game|Damage|EventAnyDamage
  (params (Damage :type Float%20%28single-precision%29) (DamageType :type Damage%20Type%20Object%20Reference) (InstigatedBy :type Controller%20Object%20Reference) (DamageCauser :type Actor%20Object%20Reference))
  (if (CallFunction|IsAlienAlive)
    (bind _alienhealth (CallFunction|DecreaseHealth Damage))
    (if (<= _alienhealth 0.0)
      (CallFunction|KillAlien)
      (Utilities|FlowControl|Delay (Variables|Default|GetKillDelay))
      (Default|IncreaseSpiderKill (Variables|Default|GetBP%20Marine))
      (Actor|DestroyActor))))

(fn ConstructionScript)

(fn IsWithinRange
  (return (< (Transformation|GetDistanceTo (Game|GetPlayerCharacter 0)) (Variables|Attack|GetAttackRange))))

(fn IsAttacking
  (return (Animation|Montage|MontageIsPlaying (Components|SkeletalMesh|GetAnimInstance (Variables|Character|GetMesh)) "/Game/Characters/Enemy_Great_Spider/Animations/SpiderAttackMontage1.SpiderAttackMontage1")))

(fn DeactivateAIMovement
  (Components|Activation|Deactivate (Variables|Character|GetCharacterMovement)))

(fn ActivateAIMovement
  (Components|Activation|Activate (Variables|Character|GetCharacterMovement) false))

(fn AttackPlayer
  (Game|Damage|ApplyDamage (Game|GetPlayerCharacter 0) (Variables|Attack|GetAttackDam) 0 0))

(fn DecreaseHealth
  (params (DamAmount :type Float%20%28single-precision%29))
  (bind _output_get (Variables|Health|SetAlienHealth (- (Variables|Health|GetAlienHealth) DamAmount)))
  (return _output_get))

(fn KillAlien
  (Variables|Default|SetDead true)
  (Movement|DeactivateAIMovement)
  (Components|Activation|SetActive (Variables|Default|GetBoxCollision) false false)
  (Collision|SetActorEnableCollision false))

(fn OutOfHealth
  (params (A :type Float%20%28single-precision%29)))

(fn IsAlienAlive
  (return (not (Variables|Default|GetDead))))